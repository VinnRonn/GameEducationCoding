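; A collision test actor that reacts when another actor begins overlapping it by moving its mesh and changing its color.
; Each overlap prints a debug message, calls MoveMesh and fires the OnColorChange event dispatcher.
; The actor binds its own ColorChange event to that dispatcher on BeginPlay, which applies a random material from the ArrayBaseColors array to CubeMesh.
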(event `self.ReceiveActorBeginOverlap`
  (params (OtherActor :type "Actor Object Reference"))
  (`KismetSystemLibrary.PrintString` (`KismetTextLibrary.Conv_TextToString` (`|FormatText` "On Trigger Overlap")) true true (struct :`G` 1.0 :`B` 0.288338 :`A` 1.0))
  (`self.MoveMesh`)
  (`self.OnColorChange`))

(event `self.ReceiveBeginPlay`
  (add `self.OnColorChange` (delegate `ColorChange`)))

(event `ColorChange`
  (`PrimitiveComponent.SetMaterial` (`self.CubeMesh`) 0 (`|GetArrayItem` (`self.ArrayBaseColors`) (`KismetMathLibrary.RandomIntegerInRange` 0 3))))

(fn `UserConstructionScript`)